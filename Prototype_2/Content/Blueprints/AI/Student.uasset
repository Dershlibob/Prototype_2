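; Student pawn in the AI folder that walks forward along its control rotation while CanMove is set.
; Each Tick it looks up all top-level MainUI widgets and adds movement input for each one, scaled by StudentSpeed, that widget's TimeSpeed and delta time.
; The game's time speed is therefore read straight from the UI, through a widget search repeated every frame.
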(event `self.ReceiveTick`
  (params (DeltaSeconds :type "Float (single-precision)"))
  (if (`self.CanMove`)
    (bind _foundwidgets (`WidgetBlueprintLibrary.GetAllWidgetsOfClass` "/Game/Blueprints/Widgets/MainUI.MainUI_C"))
    (for _array_element _foundwidgets
      (`self.AddMovementInput` (`KismetMathLibrary.GetForwardVector` (`self.GetControlRotation`)) (* DeltaSeconds (* (`self.StudentSpeed`) (`/Game/Blueprints/Widgets/MainUI.TimeSpeed` _array_element)))))))

(fn `UserConstructionScript`)