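; Door actor that the player can toggle between two rotations when interacting with it.
; Overlap with MyPlayerCharacter adds an Interact prompt widget and sets CanInteract; leaving removes the widget, clears the flag and prints a debug string.
; The InteractDoor event, not called within this Blueprint, uses a FlipFlop to snap the root's world rotation instantly, without checking CanInteract.
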(event `self.ReceiveActorBeginOverlap`
  (params (OtherActor :type "Actor Object Reference"))
  (cast `/Game/Blueprints/MyPlayerCharacter` OtherActor)
  (bind _returnvalue (`|CreateWidget` "/Game/Widgets/Interact.Interact_C"))
  (`UserWidget.AddToViewport` _returnvalue 0)
  (set `self.CanInteract` true))

(event `self.ReceiveActorEndOverlap`
  (params (OtherActor :type "Actor Object Reference"))
  (cast `/Game/Blueprints/MyPlayerCharacter` OtherActor)
  (`KismetSystemLibrary.PrintString` "Hello")
  (bind _asinteract (cast `/Game/Widgets/Interact` (stale `self.ReceiveActorBeginOverlap` _returnvalue)))
  (`Widget.RemoveFromParent` _asinteract)
  (set `self.CanInteract` false))

(event `InteractDoor`
  (bind _defaultsceneroot (`self.DefaultSceneRoot`))
  (`/Engine/EditorBlueprintResources/StandardMacros.FlipFlop`
    (:`A`
      (`SceneComponent.K2_SetWorldRotation` _defaultsceneroot (struct :`Yaw` 90.0) false false))
    (:`B`
      (`SceneComponent.K2_SetWorldRotation` :`self` _defaultsceneroot))))

(fn `UserConstructionScript`)