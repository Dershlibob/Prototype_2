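; Interactable actor where the player hands in papers to the teacher, ending the game.
; Player overlap shows an Interact widget with an F-key prompt and sets an Overlap flag, both cleared when the player leaves.
; The GivePapers event, if the player overlaps, clears all widgets, shows the GameOver widget and switches to UI-only input with a visible cursor.
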(event `self.ReceiveActorBeginOverlap`
  (params (OtherActor :type "Actor Object Reference"))
  (cast `/Game/Blueprints/Player/MyPlayerCharacter` OtherActor)
  (bind _returnvalue (`|CreateWidget` "/Game/Blueprints/Widgets/Interact.Interact_C"))
  (`UserWidget.AddToViewport` _returnvalue 0)
  (set `/Game/Blueprints/Widgets/Interact.InteractText` "Press F to hand In The Paper" _returnvalue)
  (set `self.Overlap` true))

(event `self.ReceiveActorEndOverlap`
  (params (OtherActor :type "Actor Object Reference"))
  (cast `/Game/Blueprints/Player/MyPlayerCharacter` OtherActor)
  (`Widget.RemoveFromParent` (stale `self.ReceiveActorBeginOverlap` _returnvalue))
  (set `self.Overlap` false))

(event `GivePapers`
  (bind _returnvalue (`GameplayStatics.GetPlayerController` 0))
  (if (`self.Overlap`)
    (`WidgetLayoutLibrary.RemoveAllWidgets`)
    (bind _returnvalue_2 (`|CreateWidget` "/Game/Blueprints/Widgets/GameOver.GameOver_C"))
    (`UserWidget.AddToViewport` _returnvalue_2 0)
    (`WidgetBlueprintLibrary.SetInputMode_UIOnlyEx` _returnvalue _returnvalue_2)
    (set `PlayerController.bShowMouseCursor` true _returnvalue)))

(fn `UserConstructionScript`)