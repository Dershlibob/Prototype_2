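; Teacher's coffee pickup that shows an "F" interact prompt widget while the player character overlaps it.
; The DrinkCoffee event, not triggered within this Blueprint, destroys the actor if overlapped, halves TimeSpeed on the MainUI widget and shows a SpeedyBoi widget.
; A Delay is meant to restore normal TimeSpeed afterwards, but it runs on the already destroyed actor, so the reset likely never fires.
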(event `self.ReceiveActorBeginOverlap`
  (params (OtherActor :type "Actor Object Reference"))
  (cast `/Game/Blueprints/Player/MyPlayerCharacter` OtherActor)
  (set `self.Overlapping` true)
  (bind _returnvalue (`|CreateWidget` "/Game/Blueprints/Widgets/Interact.Interact_C"))
  (`UserWidget.AddToViewport` _returnvalue 0)
  (set `/Game/Blueprints/Widgets/Interact.InteractText` "Press F to Drink Teacher's Coffee" _returnvalue))

(event `self.ReceiveActorEndOverlap`
  (params (OtherActor :type "Actor Object Reference"))
  (cast `/Game/Blueprints/Player/MyPlayerCharacter` OtherActor)
  (`Widget.RemoveFromParent` (stale `self.ReceiveActorBeginOverlap` _returnvalue))
  (set `self.Overlapping` false))

(event `DrinkCoffee`
  (if (`self.Overlapping`)
    (`self.K2_DestroyActor`)
    (bind _foundwidgets (`WidgetBlueprintLibrary.GetAllWidgetsOfClass` "/Game/Blueprints/Widgets/MainUI.MainUI_C"))
    (for _array_element _foundwidgets
      (set `/Game/Blueprints/Widgets/MainUI.TimeSpeed` 0.5 _array_element)
      (bind _returnvalue (`|CreateWidget` "/Game/Blueprints/Widgets/SpeedyBoi.SpeedyBoi_C"))
      (`UserWidget.AddToViewport` _returnvalue 0)
      (`KismetSystemLibrary.Delay` 30.0)
      (set `/Game/Blueprints/Widgets/MainUI.TimeSpeed` 1.0 _array_element))))

(fn `UserConstructionScript`)