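; Interactable door that toggles open and closed and releases Student actors to move when it opens.
; Player overlap shows an interact prompt widget and sets CanInteract; leaving removes the prompt, clears the flag and prints a debug string.
; InteractDoor, with no caller in this graph, uses a FlipFlop to snap the root between two fixed world rotations, enabling CanMove on every Student on the opening branch only.
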(event `self.ReceiveActorBeginOverlap`
  (params (OtherActor :type "Actor Object Reference"))
  (cast `/Game/Blueprints/Player/MyPlayerCharacter` OtherActor)
  (bind _returnvalue (`|CreateWidget` "/Game/Blueprints/Widgets/Interact.Interact_C"))
  (`UserWidget.AddToViewport` _returnvalue 0)
  (set `/Game/Blueprints/Widgets/Interact.InteractText` "Press F to Interact" _returnvalue)
  (set `self.CanInteract` true))

(event `self.ReceiveActorEndOverlap`
  (params (OtherActor :type "Actor Object Reference"))
  (cast `/Game/Blueprints/Player/MyPlayerCharacter` OtherActor)
  (`KismetSystemLibrary.PrintString` "Hello")
  (bind _asinteract (cast `/Game/Blueprints/Widgets/Interact` (stale `self.ReceiveActorBeginOverlap` _returnvalue)))
  (`Widget.RemoveFromParent` _asinteract)
  (set `self.CanInteract` false))

(event `InteractDoor`
  (bind _defaultsceneroot (`self.DefaultSceneRoot`))
  (`/Engine/EditorBlueprintResources/StandardMacros.FlipFlop`
    (:`A`
      (`SceneComponent.K2_SetWorldRotation` _defaultsceneroot (struct :`Yaw` 90.0) false false)
      (bind _outactors (`GameplayStatics.GetAllActorsOfClass` "/Game/Blueprints/AI/Student.Student_C"))
      (for _array_element _outactors
        (set `/Game/Blueprints/AI/Student.CanMove` true _array_element)))
    (:`B`
      (`SceneComponent.K2_SetWorldRotation` :`self` _defaultsceneroot))))

(fn `UserConstructionScript`)