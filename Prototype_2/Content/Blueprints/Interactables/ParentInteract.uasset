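; ParentInteract is an interactable actor, apparently a base for collectable paper items, that feeds the player's item counters.
; Every Tick it loops over all MyPlayerCharacter actors, incrementing Collectables and setting RemainingItems to the current count of ParentInteract actors.
; These updates poll with GetAllActorsOfClass each frame, so Collectables rises continuously rather than per pickup.
; The DestroyPaper event destroys the actor only while Overlapping is true.
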(event `self.ReceiveTick`
  (params (DeltaSeconds :type "Float (single-precision)"))
  (bind _outactors (`GameplayStatics.GetAllActorsOfClass` "/Game/Blueprints/Player/MyPlayerCharacter.MyPlayerCharacter_C"))
  (for _array_element _outactors
    (set `/Game/Blueprints/Player/MyPlayerCharacter.Collectables` (+ (`/Game/Blueprints/Player/MyPlayerCharacter.Collectables` _array_element) 1) _array_element)
    (bind _outactors_2 (`GameplayStatics.GetAllActorsOfClass` "ParentInteract_C"))
    (set `/Game/Blueprints/Player/MyPlayerCharacter.RemainingItems` (`KismetArrayLibrary.Array_Length` _outactors_2) _array_element)))

(event `DestroyPaper`
  (if (`self.Overlapping`)
    (`self.K2_DestroyActor`)))

(fn `UserConstructionScript`)