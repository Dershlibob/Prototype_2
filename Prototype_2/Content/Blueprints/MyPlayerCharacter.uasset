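; Player character Blueprint with axis-driven movement and look, plus a push interaction for doors.
; Tick sets the arms' Animation Blueprint walking flag from movement input and prints debug speed and push state.
; Pressing Push searches all Door actors, calls InteractDoor on interactable ones, and triggers PushAnim, which holds the pushing flag for a fixed delay.
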(event `self.ReceiveTick`
  (params (DeltaSeconds :type "Float (single-precision)"))
  (`|ExecutionSequence`
    (:`then_0`
      (`KismetSystemLibrary.PrintString` (`KismetStringLibrary.Conv_IntToString` (`KismetMathLibrary.FTrunc` (`KismetMathLibrary.VSize` (`self.GetVelocity`)))) true true (struct :`G` 0.66 :`B` 1.0 :`A` 1.0) DeltaSeconds))
    (:`then_1`
      ;[1 1 1] Animations
      (if (or (!= (`self.GetInputAxisValue`) 0.0) (!= (`self.GetInputAxisValue`) 0.0))
        (bind _asabp (cast `/Game/Blueprints/ABP` (`SkeletalMeshComponent.GetAnimInstance` (`self.CharacterArms`))))
        (set `/Game/Blueprints/ABP.IsWalking` true _asabp)
        (else
          (bind _asabp_2 (cast `/Game/Blueprints/ABP` (`SkeletalMeshComponent.GetAnimInstance` (`self.CharacterArms`))))
          (set `/Game/Blueprints/ABP.IsWalking` false _asabp_2))))
    (:`then_2`
      (`KismetSystemLibrary.PrintString` (`KismetStringLibrary.Conv_BoolToString` (`/Game/Blueprints/ABP.IsPushing` (stale `PushAnim` _asabp))) true true (struct :`G` 0.66 :`B` 1.0 :`A` 1.0) 0.001))))

(event `InputAxis|Forward_Backward`
  (params (AxisValue :type "Float (single-precision)"))
  ;[1 1 1] Movement Inputs
  (`self.AddMovementInput` (`KismetMathLibrary.GetForwardVector` (`self.GetControlRotation`)) AxisValue))

(event `InputAxis|RotateLeftRight`
  (params (AxisValue :type "Float (single-precision)"))
  ;[1 1 1] Camera axis inputs
  (`self.AddControllerYawInput` AxisValue))

(event `InputAxis|Look_Up_Down`
  (params (AxisValue :type "Float (single-precision)"))
  ;[1 1 1] Camera axis inputs
  (`self.AddControllerPitchInput` AxisValue))

(event `InputAxis|Left_Right`
  (params (AxisValue :type "Float (single-precision)"))
  ;[1 1 1] Movement Inputs
  (`self.AddMovementInput` (`KismetMathLibrary.GetRightVector` (`self.GetControlRotation`)) AxisValue))

(event `InputAction|Push`
  (params (Key :type "Key Structure"))
  ;[1 1 1] Play Push Animation
  ;;[1 1 1] F key
  (:`Pressed`
    (bind _outactors (`GameplayStatics.GetAllActorsOfClass` "/Game/Blueprints/Door.Door_C"))
    (for _array_element _outactors
      (if (`/Game/Blueprints/Door.CanInteract` _array_element)
        (`/Game/Blueprints/Door.InteractDoor` _array_element)
        (`self.PushAnim`)))))

(event `PushAnim`
  (bind _asabp (cast `/Game/Blueprints/ABP` (`SkeletalMeshComponent.GetAnimInstance` (`self.CharacterArms`))))
  (if (not (`/Game/Blueprints/ABP.IsPushing` _asabp))
    (set `/Game/Blueprints/ABP.IsPushing` true _asabp)
    (`KismetSystemLibrary.Delay` 1.3)
    (set `/Game/Blueprints/ABP.IsPushing` false _asabp)))

(fn `UserConstructionScript`)