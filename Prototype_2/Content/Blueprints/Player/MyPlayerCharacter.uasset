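; First-person-style player character that walks, looks around and interacts with coffee, papers, a teacher hand-in actor and doors.
; Axis inputs drive control-rotation-relative movement and camera; Tick sets the arms AnimBP's walking flag and recounts remaining Paper actors.
; Push calls the interaction function on every Coffee, Paper and hand-in actor, but checks CanInteract on doors.
; Only door interactions trigger the arms' push animation, held by a timed flag.
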(event `self.ReceiveTick`
  (params (DeltaSeconds :type "Float (single-precision)"))
  (`|ExecutionSequence`
    (:`then_0`
      ;[1 1 1] Animations
      (if (or (!= (`self.GetInputAxisValue`) 0.0) (!= (`self.GetInputAxisValue`) 0.0))
        (bind _asabp (cast `/Game/Blueprints/Player/ABP` (`SkeletalMeshComponent.GetAnimInstance` (`self.CharacterArms`))))
        (set `/Game/Blueprints/Player/ABP.IsWalking` true _asabp)
        (else
          (bind _asabp_2 (cast `/Game/Blueprints/Player/ABP` (`SkeletalMeshComponent.GetAnimInstance` (`self.CharacterArms`))))
          (set `/Game/Blueprints/Player/ABP.IsWalking` false _asabp_2))))
    (:`then_1`
      (bind _outactors (`GameplayStatics.GetAllActorsOfClass` "/Game/Blueprints/Interactables/ItemsToInteract/Paper.Paper_C"))
      (set `self.RemainingItems` (`KismetArrayLibrary.Array_Length` _outactors)))))

(event `InputAxis|Forward_Backward`
  (params (AxisValue :type "Float (single-precision)"))
  ;[1 1 1] Movement Inputs
  (`self.AddMovementInput` (`KismetMathLibrary.GetForwardVector` (`self.GetControlRotation`)) (* AxisValue (`self.Speed`))))

(event `InputAxis|RotateLeftRight`
  (params (AxisValue :type "Float (single-precision)"))
  ;[1 1 1] Camera axis inputs
  (`self.AddControllerYawInput` AxisValue))

(event `InputAxis|Look_Up_Down`
  (params (AxisValue :type "Float (single-precision)"))
  ;[1 1 1] Camera axis inputs
  (`self.AddControllerPitchInput` AxisValue))

(event `InputAxis|Left_Right`
  (params (AxisValue :type "Float (single-precision)"))
  ;[1 1 1] Movement Inputs
  (`self.AddMovementInput` (`KismetMathLibrary.GetRightVector` (`self.GetControlRotation`)) (* AxisValue (`self.Speed`))))

(event `InputAction|Push`
  (params (Key :type "Key Structure"))
  ;[1 1 1] F key
  (:`Pressed`
    (bind _outactors (`GameplayStatics.GetAllActorsOfClass` "/Game/Blueprints/Interactables/Coffee.Coffee_C"))
    (for _array_element _outactors
      (`/Game/Blueprints/Interactables/Coffee.DrinkCoffee` _array_element))
    (bind _outactors_2 (`GameplayStatics.GetAllActorsOfClass` "/Game/Blueprints/Interactables/ItemsToInteract/Paper.Paper_C"))
    ;[1 1 1] Play Push Animation
    (for _array_element_2 _outactors_2
      (`/Game/Blueprints/Interactables/ParentInteract.DestroyPaper` _array_element_2))
    (bind _outactors_3 (`GameplayStatics.GetAllActorsOfClass` "/Game/Blueprints/Interactables/BPgivePapersToTeacher.BPgivePapersToTeacher_C"))
    (for _array_element_3 _outactors_3
      (`/Game/Blueprints/Interactables/BPgivePapersToTeacher.GivePapers` _array_element_3))
    (bind _outactors_4 (`GameplayStatics.GetAllActorsOfClass` "/Game/Blueprints/Interactables/Door.Door_C"))
    (for _array_element_4 _outactors_4
      (if (`/Game/Blueprints/Interactables/Door.CanInteract` _array_element_4)
        (`/Game/Blueprints/Interactables/Door.InteractDoor` _array_element_4)
        (`self.PushAnim`)))))

(event `PushAnim`
  (bind _asabp (cast `/Game/Blueprints/Player/ABP` (`SkeletalMeshComponent.GetAnimInstance` (`self.CharacterArms`))))
  (if (not (`/Game/Blueprints/Player/ABP.IsPushing` _asabp))
    (set `/Game/Blueprints/Player/ABP.IsPushing` true _asabp)
    (`KismetSystemLibrary.Delay` 1.3)
    (set `/Game/Blueprints/Player/ABP.IsPushing` false _asabp)))

(fn `UserConstructionScript`)